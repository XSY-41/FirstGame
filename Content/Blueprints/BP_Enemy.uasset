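; BP_Enemy is an enemy character that reacts to damage and collapses when its health runs out.
; AnyDamage subtracts the incoming damage from Health.
; At zero or below, it turns on physics simulation for the mesh; otherwise it launches the character slightly upward and along its own forward vector as a hit reaction.
; It has no other active logic.
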(event `self.ReceiveAnyDamage`
  (params (Damage :type "Float (single-precision)") (DamageType :type "DamageType Object Reference") (InstigatedBy :type "Controller Object Reference") (DamageCauser :type "Actor Object Reference"))
  (bind _output_get (set `self.Health` (- (`self.Health`) Damage)))
  (if (<= _output_get 0.0)
    (`PrimitiveComponent.SetSimulatePhysics` (`self.Mesh`) true)
    (else
      (`self.LaunchCharacter` (+ (* (`self.GetActorForwardVector`) 200.0) (* (`self.GetActorUpVector`) 100.0))))))

(fn `UserConstructionScript`)